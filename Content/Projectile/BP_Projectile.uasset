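; BP_Projectile is a projectile actor that homes in on an AI character along a curved path.
; On BeginPlay it stores the first NMAICharacter found in the level as its target.
; Each Tick it moves at constant speed along the target direction rotated by a fixed yaw offset, producing a spiral-like approach.
; Movement has no sweep, and there is no hit logic; the time accumulator is disconnected.
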(event Collision|EventActorBeginOverlap
  (params (OtherActor :type Actor%20Object%20Reference)))

(event EventTick
  (params (DeltaSeconds :type Float%20%28single-precision%29))
  (Transformation|SetActorLocation (+ (Transformation|GetActorLocation) (* (Math|Vector|RotateVectorAroundAxis (Math|Vector|Normalize (- (Transformation|GetActorLocation (Variables|Default|GetTarget)) (Transformation|GetActorLocation))) 3e+01 "0.000000,0.000000,1.000000") 5e+02 DeltaSeconds)) false false))

(event EventBeginPlay
  (bind _outactors (Actor|GetAllActorsOfClass "/Script/NewMoon.NMAICharacter"))
  (Variables|Default|SetTarget (Utilities|Array|Get(acopy) _outactors)))

(fn ConstructionScript)