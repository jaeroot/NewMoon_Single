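; BP_CircularDecal is a test actor that animates a circular decal growing over a set time.
; BeginPlay creates a dynamic material instance on the Decal component and sets its SectorCount parameter.
; Tick accumulates delta time until RangeTime is reached, mapping it linearly with a clamped range to the material's Radius parameter, so the growth plays once.
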(event EventBeginPlay
  (bind _returnvalue (Rendering|Material|CreateDynamicMaterialInstance (Variables|Default|GetDecal) :!class /Script/Engine.DecalComponent))
  (Rendering|Material|SetScalarParameterValue _returnvalue "SectorCount" 4.0 :!class /Script/Engine.MaterialInstanceDynamic))

(event Collision|EventActorBeginOverlap
  (params (OtherActor :type Actor%20Object%20Reference)))

(event EventTick
  (params (DeltaSeconds :type Float%20%28single-precision%29))
  (if (< (Variables|Default|GetRangeTimeAcc) (Variables|Default|GetRangeTime))
    (bind _output_get (Variables|Default|SetRangeTimeAcc (+ (Variables|Default|GetRangeTimeAcc) DeltaSeconds)))
    (Rendering|Material|SetScalarParameterValue (stale EventBeginPlay _returnvalue) "Radius" (Math|Float|MapRangeClamped _output_get 0.0 (Variables|Default|GetRangeTime) 0.0 0.5) :!class /Script/Engine.MaterialInstanceDynamic)))

(fn ConstructionScript)