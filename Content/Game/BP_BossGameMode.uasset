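; BP_BossGameMode is the game mode for the boss level, preparing the player, timing the fight and handling stage clear.
; On BeginPlay it enables kick, fireball and guard on the NMPlayerCharacter and flags it as being in a boss level.
; Tick accumulates ClearTime.
; ClearStage shows the WBP_Result4 screen with UI-only input and a mouse cursor, then freezes the game via zero global time dilation.
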(event EventBeginPlay
  (bind _asnmplayer_character (Utilities|Casting|CastToNMPlayerCharacter (Pawn|GetControlledPawn (Game|GetPlayerController 0))))
  (Variables|/Script/NewMoon.NMPlayerCharacter|SetbCanKick _asnmplayer_character true)
  (Variables|/Script/NewMoon.NMPlayerCharacter|SetbCanFireBall _asnmplayer_character true)
  (Variables|/Script/NewMoon.NMPlayerCharacter|SetbCanGuard _asnmplayer_character true)
  (Variables|/Script/NewMoon.NMPlayerCharacter|SetbIsBossLevel _asnmplayer_character true))

(event EventTick
  (params (DeltaSeconds :type Float%20%28single-precision%29))
  (Variables|Default|SetClearTime (+ (Variables|Default|GetClearTime) DeltaSeconds)))

(fn ConstructionScript)

(fn ClearStage
  (bind _returnvalue (Game|GetPlayerController 0))
  (bind _returnvalue_2 (UserInterface|CreateWidget "/Game/UI/InGame/WBP_Result4.WBP_Result4_C" (Game|GetPlayerController 0)))
  (UserInterface|Viewport|AddtoViewport _returnvalue_2 0)
  (Input|SetInputModeUIOnly _returnvalue _returnvalue_2 "DoNotLock" false)
  (Variables|/Script/Engine.PlayerController|SetbShowMouseCursor _returnvalue true)
  (Utilities|Time|SetGlobalTimeDilation 0.0))