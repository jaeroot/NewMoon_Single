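; Game mode Blueprint that handles stage completion, rewarding the player and showing a result screen.
; ClearStage switches on stage number 1 to 3, unlocking kick, fireball or guard on NMPlayerCharacter; the first two stages also move its resurrect point.
; Each stage adds its own result widget, then shares a tail that sets UI-only input, shows the cursor and freezes time via zero dilation.
; The shared tail always focuses the stage 2 widget.
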(event EventBeginPlay)

(event EventTick
  (params (DeltaSeconds :type Float%20%28single-precision%29)))

(fn ConstructionScript)

(fn ClearStage
  (params (StageCount :type Integer))
  (bind _returnvalue (Game|GetPlayerController 0))
  (bind _returnvalue_2 (Game|GetPlayerController 0))
  (bind _returnvalue_3 (Pawn|GetControlledPawn _returnvalue_2))
  (switch int StageCount
    (:1
      (bind _asnmplayer_character (Utilities|Casting|CastToNMPlayerCharacter _returnvalue_3))
      (Variables|/Script/NewMoon.NMPlayerCharacter|SetbCanKick _asnmplayer_character true)
      (Variables|/Script/NewMoon.NMPlayerCharacter|SetResurrectLocation _asnmplayer_character "-5780.000000,-990.000000,269.397958")
      (Variables|/Script/NewMoon.NMPlayerCharacter|SetResurrectRotation _asnmplayer_character "0.000000,-90.000000,0.000000")
      (bind _returnvalue_4 (UserInterface|CreateWidget "/Game/UI/InGame/WBP_Result1.WBP_Result1_C"))
      (UserInterface|Viewport|AddtoViewport _returnvalue_4 0))
    (:2
      (bind _asnmplayer_character_2 (Utilities|Casting|CastToNMPlayerCharacter _returnvalue_3))
      (Variables|/Script/NewMoon.NMPlayerCharacter|SetbCanFireBall _asnmplayer_character_2 true)
      (Variables|/Script/NewMoon.NMPlayerCharacter|SetResurrectLocation _asnmplayer_character_2 "-4590.000000,400.000000,219.397958")
      (Variables|/Script/NewMoon.NMPlayerCharacter|SetResurrectRotation _asnmplayer_character_2 "0.000000,180.000000,0.000000")
      (bind _returnvalue_5 (UserInterface|CreateWidget "/Game/UI/InGame/WBP_Result2.WBP_Result2_C" _returnvalue_2))
      (UserInterface|Viewport|AddtoViewport _returnvalue_5 0))
    (:3
      (bind _asnmplayer_character_3 (Utilities|Casting|CastToNMPlayerCharacter _returnvalue_3))
      (Variables|/Script/NewMoon.NMPlayerCharacter|SetbCanGuard _asnmplayer_character_3 true)
      (bind _returnvalue_6 (UserInterface|CreateWidget "/Game/UI/InGame/WBP_Result3.WBP_Result3_C"))
      (UserInterface|Viewport|AddtoViewport _returnvalue_6 0)))
  (Input|SetInputModeUIOnly _returnvalue _returnvalue_5 "DoNotLock" false)
  (Variables|/Script/Engine.PlayerController|SetbShowMouseCursor _returnvalue true)
  (Utilities|Time|SetGlobalTimeDilation 0.0))