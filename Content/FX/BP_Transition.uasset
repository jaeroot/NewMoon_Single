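; Level transition trigger that sends the player to the Demonstration_Castle level once the guard, fireball and kick abilities are all available.
; Tick polls the player character's three ability flags, then shows the PLevelUpDetail2 component and sets an Activate flag that is never cleared here.
; While activated, a player character beginning overlap with the Box opens the castle level.
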(event OnComponentBeginOverlap(Box)
  (params (OverlappedComponent :type Primitive%20Component%20Object%20Reference) (OtherActor :type Actor%20Object%20Reference) (OtherComp :type Primitive%20Component%20Object%20Reference) (OtherBodyIndex :type Integer) (bFromSweep :type Boolean) (SweepResult :type Hit%20Result%20Structure%20%28by%20ref%29))
  (if (Variables|Default|GetActivate?)
    (Utilities|Casting|CastToNMPlayerCharacter OtherActor)
    (Game|OpenLevel(byObjectReference) "/Game/FantasyBundle/Maps/Demonstration_Castle.Demonstration_Castle")))

(event EventBeginPlay)

(event Collision|EventActorBeginOverlap
  (params (OtherActor :type Actor%20Object%20Reference)))

(event EventTick
  (params (DeltaSeconds :type Float%20%28single-precision%29))
  (bind _asnmplayer_character (Utilities|Casting|CastToNMPlayerCharacter (Game|GetPlayerCharacter 0)))
  (if (Math|Boolean|ANDBoolean (Variables|/Script/NewMoon.NMPlayerCharacter|GetbCanGuard _asnmplayer_character) (Variables|/Script/NewMoon.NMPlayerCharacter|GetbCanFireBall _asnmplayer_character) (Variables|/Script/NewMoon.NMPlayerCharacter|GetbCanKick _asnmplayer_character))
    (Rendering|SetVisibility (Variables|Default|GetP_levelUp_Detail2) true false)
    (Variables|Default|SetActivate? true)))

(fn ConstructionScript)